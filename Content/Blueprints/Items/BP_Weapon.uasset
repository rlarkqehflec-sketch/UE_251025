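; BP_Weapon is an equippable weapon item that runs its parent pickup logic, then has the player equip it.
; Shoot line-traces on the Visibility channel from the screen center to find the aim point.
; It then spawns an actor at the mesh's Muzzle socket, rotated toward the impact point, so shots converge on the center of the view, with no fallback when the trace misses.
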(event `self.Pickup`
  (params (Player :type "/Game/Blueprints/Characters/BP_Player Object Reference"))
  (`parent.Pickup` null)
  (`/Game/Blueprints/Characters/BP_Player.Equip` Player self))

(event `Shoot`
  (bind (_returnvalue_x _returnvalue_y) (`KismetMathLibrary.BreakVector2D` (`WidgetLayoutLibrary.GetViewportSize`)))
  (bind (_returnvalue_location _returnvalue_rotation _returnvalue_scale) (`KismetMathLibrary.BreakTransform` (`SceneComponent.GetSocketTransform` (`self.SkeletalMesh`) "Muzzle" "RTS_World")))
  (bind (_worldposition _worlddirection) (`GameplayStatics.DeprojectScreenToWorld` (`GameplayStatics.GetPlayerController` 0) (`KismetMathLibrary.MakeVector2D` (/ _returnvalue_x 2.0) (/ _returnvalue_y 2.0))))
  (bind _outhit (`KismetSystemLibrary.LineTraceSingle` _worldposition (+ _worldposition (* _worlddirection 10000.0)) "TraceTypeQuery1"))
  (`|SpawnActorFromClass` "/Game/Blueprints/Items/BP_Projectile.BP_Projectile_C" (`KismetMathLibrary.MakeTransform` _returnvalue_location (`KismetMathLibrary.Conv_VectorToRotator` (`KismetMathLibrary.Normal` (- (`.ImpactPoint` (`GameplayStatics.BreakHitResult` _outhit)) _returnvalue_location))) _returnvalue_scale) "Undefined" "MultiplyWithRoot" null null))

(fn `UserConstructionScript`
  (`parent.UserConstructionScript`))