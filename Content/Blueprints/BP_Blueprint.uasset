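; BP_Blueprint is a simple actor that moves itself forward continuously, apparently a transform-node experiment.
; BeginPlay nudges it along world X, then Tick steps it along its forward vector by a fixed amount per frame, so speed depends on frame rate.
; Both moves skip sweeping.
; Rotation and scale setters and other direction vectors are left unwired, and the overlap event and construction script are empty.
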(event `self.ReceiveBeginPlay`
  (`self.K2_SetActorLocation` (+ (`self.K2_GetActorLocation`) (100.0 0.0 0.0))))

(event `self.ReceiveTick`
  (params (DeltaSeconds :type "Float (single-precision)"))
  (`self.K2_SetActorLocation` (+ (`self.K2_GetActorLocation`) (* (`self.GetActorForwardVector`) 3.0))))

(fn `UserConstructionScript`)