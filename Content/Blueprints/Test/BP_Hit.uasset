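; BP_Hit is a test actor whose point light switches on and off when the player hits its box.
; The light intensity is zeroed at BeginPlay.
; Each Box component hit from a BP_Player reads the Toggle boolean, sets the intensity to bright or zero accordingly, then flips the boolean.
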(event `self.ReceiveBeginPlay`
  (`LightComponent.SetIntensity` (`self.PointLight`) 0.0))

(event `self.Box.OnComponentHit`
  (params (HitComponent :type "PrimitiveComponent Object Reference") (OtherActor :type "Actor Object Reference") (OtherComp :type "PrimitiveComponent Object Reference") (NormalImpulse :type "Vector Structure") (Hit :type "HitResult Structure (by ref)"))
  (cast `/Game/Blueprints/Characters/BP_Player` OtherActor)
  (if (`self.Toggle`)
    (`LightComponent.SetIntensity` (`self.PointLight`) 5000.0)
    (set `self.Toggle` false)
    (else
      (`LightComponent.SetIntensity` (`self.PointLight`) 0.0)
      (set `self.Toggle` true))))

(fn `UserConstructionScript`)